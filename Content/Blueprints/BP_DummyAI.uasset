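; BP_DummyAI is an enemy character with health, a floating health bar and a burst rifle.
; On BeginPlay it spawns the rifle attached to the hand_r socket and links the health bar widget to itself.
; StartShooting and StopShooting events toggle weapon fire.
; Damage updates the bar and plays a hit-react montage, or on death ragdolls the mesh, hides the bar and destroys the actor after a delay.
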(event `self.ReceiveBeginPlay`
  ;[1 1 1] OnBeginPlay
  (`self.Initialize Weapon`)
  (bind _healthbarref (`self.InitializeHealthBarWidget`))
  (set `/Game/UI/WBP_EnemyHealthBar.Enemy` self _healthbarref)
  (`/Game/UI/WBP_EnemyHealthBar.UpdateHealth` _healthbarref))

(event `StartShooting`
  (`/Game/Blueprints/Weapons/BP_Weapon_Enemy_BurstRifle.StartFiring` (`self.EnemyWeapon`)))

(event `StopShooting`
  (bind _enemyweapon (`self.EnemyWeapon`))
  (set `/Game/Blueprints/Weapons/BP_Weapon_Enemy_BurstRifle.IsFiring` false _enemyweapon)
  (`/Game/Blueprints/Weapons/BP_Weapon.TurnOffFX&Audio` _enemyweapon))

(event `self.ReceiveAnyDamage`
  (params (Damage :type "Float (single-precision)") (DamageType :type "DamageType Object Reference") (InstigatedBy :type "Controller Object Reference") (DamageCauser :type "Actor Object Reference"))
  ;[1 1 1] Lose Health
  (bind _output_get (set `self.Health` (- (`self.Health`) Damage)))
  (`/Game/UI/WBP_EnemyHealthBar.UpdateHealth` (`self.As WBP Enemy Health Bar`))
  ;;[1 1 1] If Enemy is dead
  (bind _output_get_2 (set `self.IsDead` (<= _output_get 0.0)))
  (if _output_get_2
    (`PrimitiveComponent.SetSimulatePhysics` (`self.Mesh`) true)
    (`Widget.SetVisibility` (`self.As WBP Enemy Health Bar`) "Collapsed")
    (`KismetSystemLibrary.Delay` 3.0)
    (`self.K2_DestroyActor`)
    (else
      ;;[1 1 1] Animacao de hit
      (`|PlayMontage` (`self.Mesh`) "/Game/AnimStarterPack/AM_HitReact3.AM_HitReact3"))))

(fn `Initialize Weapon`
  (bind _weapon (`self.Weapon`))
  (bind _returnvalue (`|SpawnActorFromClass` "/Game/Blueprints/Weapons/BP_Weapon_Enemy_BurstRifle.BP_Weapon_Enemy_BurstRifle_C" (`KismetMathLibrary.MakeTransform` (`SceneComponent.K2_GetComponentLocation` _weapon)) "AlwaysSpawn" "OverrideRootScale" null null))
  (bind _output_get (set `self.EnemyWeapon` _returnvalue))
  (`self.K2_AttachToComponent` _output_get _weapon "hand_r" "SnapToTarget" "SnapToTarget" "KeepRelative" true))

(fn `InitializeHealthBarWidget`
  (returns (HealthBarRef :type "/Game/UI/WBP_EnemyHealthBar Object Reference"))
  (bind _aswbp_enemy_health_bar (cast `/Game/UI/WBP_EnemyHealthBar` (`WidgetComponent.GetUserWidgetObject` (`self.EnemyHealthBar`))))
  (bind _output_get (set `self.As WBP Enemy Health Bar` _aswbp_enemy_health_bar))
  (return _output_get))

(fn `UserConstructionScript`)