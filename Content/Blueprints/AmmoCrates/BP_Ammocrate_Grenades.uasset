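; Grenade ammo crate pickup that refills the player's grenade holster on overlap.
; When a BP_FPSCharacter overlaps it while below max grenade capacity, it adds AmmoToAdd to the holster count, prints a debug message and destroys itself.
; The added amount is not clamped to the maximum.
; CanPickup and IsHolsterFull hold unused weapon-capacity checks that the overlap logic does not call.
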(event `self.ReceiveActorBeginOverlap`
  (params (OtherActor :type "Actor Object Reference"))
  (bind _asbp_fpscharacter (cast `/Game/Blueprints/BP_FPSCHaracter` OtherActor))
  (bind _output_get (set `self.FPSPlayerRef` _asbp_fpscharacter))
  (bind _currentgrenadeholsteramount (`/Game/Blueprints/BP_FPSCHaracter.CurrentGrenadeHolsterAmount` _output_get))
  (if (< _currentgrenadeholsteramount (`/Game/Blueprints/BP_FPSCHaracter.MaxGrenadeCapacity` _output_get))
    (`KismetSystemLibrary.PrintString` "Grenade Collected" true true (struct :`R` 1.0 :`G` 0.357946 :`A` 1.0))
    (set `/Game/Blueprints/BP_FPSCHaracter.CurrentGrenadeHolsterAmount` (+ _currentgrenadeholsteramount (`self.AmmoToAdd`)) _output_get)
    (`self.K2_DestroyActor`)))

(fn `UserConstructionScript`
  (`parent.UserConstructionScript`))