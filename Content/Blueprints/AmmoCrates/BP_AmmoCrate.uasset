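; BP_AmmoCrate is a pickup that adds reserve (holster) ammo to the FPS player character on overlapping its box.
; Overlap caches the player and calls PickupAmmo, which requires the current weapon's holster to have room for at least one full clip.
; On success it adds AmmoToAdd to the crate's WeaponInUse slot, which can differ from the checked weapon, then prints a message and destroys itself.
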(event `self.Box.OnComponentBeginOverlap`
  (params (OverlappedComponent :type "PrimitiveComponent Object Reference") (OtherActor :type "Actor Object Reference") (OtherComp :type "PrimitiveComponent Object Reference") (OtherBodyIndex :type Integer) (bFromSweep :type Boolean) (SweepResult :type "HitResult Structure (by ref)"))
  ;[1 1 1] Get Player Ref
  (bind _asbp_fpscharacter (cast `/Game/Blueprints/BP_FPSCHaracter` OtherActor))
  (bind _output_get (set `self.FPSPlayerRef` _asbp_fpscharacter))
  (`self.PickupAmmo` _output_get (`self.WeaponInUse`)))

(event `self.Box.OnComponentEndOverlap`
  (params (OverlappedComponent :type "PrimitiveComponent Object Reference") (OtherActor :type "Actor Object Reference") (OtherComp :type "PrimitiveComponent Object Reference") (OtherBodyIndex :type Integer))
  ;[1 1 1] Get Player Ref
  (set `self.FPSPlayerRef` null))

(fn `CheckIfHolsterIsFull`
  (returns (IsFull :type Boolean))
  (bind _fpsplayerref (`self.FPSPlayerRef`))
  (return (>= (`|GetArrayItem` (`/Game/Blueprints/BP_FPSCHaracter.CurrentHolsterAmount` _fpsplayerref) (`/Game/Blueprints/BP_FPSCHaracter.WeaponIndex` _fpsplayerref)) (`/Game/Blueprints/Weapons/BP_Weapon.MaxHolsterCapacity` (`/Game/Blueprints/BP_FPSCHaracter.CurrentSelectedWeapon` _fpsplayerref)))))

(fn `CheckIfPlayerCanPickupTheAmmoCrate`
  (returns (CanPickup :type Boolean))
  (bind _fpsplayerref (`self.FPSPlayerRef`))
  (bind _currentselectedweapon (`/Game/Blueprints/BP_FPSCHaracter.CurrentSelectedWeapon` _fpsplayerref))
  (bind _isfull (`self.CheckIfHolsterIsFull`))
  (return (and (not _isfull) (<= (`|GetArrayItem` (`/Game/Blueprints/BP_FPSCHaracter.CurrentHolsterAmount` _fpsplayerref) (`/Game/Blueprints/BP_FPSCHaracter.WeaponIndex` _fpsplayerref)) (- (`/Game/Blueprints/Weapons/BP_Weapon.MaxHolsterCapacity` _currentselectedweapon) (`/Game/Blueprints/Weapons/BP_Weapon.MaxClipCapacity` _currentselectedweapon))))))

(fn `PickupAmmo`
  (params (Player :type "/Game/Blueprints/BP_FPSCHaracter Object Reference") (WeaponInUse :type Integer))
  (bind _currentholsteramount (`/Game/Blueprints/BP_FPSCHaracter.CurrentHolsterAmount` Player))
  (bind _weaponinuse (`local.WeaponInUse`))
  (bind _canpickup (`self.CheckIfPlayerCanPickupTheAmmoCrate`))
  (if _canpickup
    (`KismetSystemLibrary.PrintString` "Ammo Collected" true true (struct :`R` 1.0 :`G` 0.357946 :`A` 1.0))
    (`KismetArrayLibrary.Array_Set` _currentholsteramount _weaponinuse (+ (`|GetArrayItem` _currentholsteramount _weaponinuse) (`self.AmmoToAdd`)))
    (`self.K2_DestroyActor`)))

(fn `UserConstructionScript`)