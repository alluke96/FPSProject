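; Behavior tree task that advances the patrol path index for a BP_Dummy pawn moving forward along its PatrolPath.
; When the blackboard direction is forward and a next path point exists, it increments the index and finishes successfully.
; At the last point it flips the direction to reverse and fails; it also fails without changes when the direction is not forward.
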(event `self.ReceiveExecuteAI`
  (params (OwnerController :type "AIController Object Reference") (ControlledPawn :type "Pawn Object Reference"))
  (bind _bb_direction (`self.BB_Direction`))
  (bind _returnvalue (+ (`BTFunctionLibrary.GetBlackboardValueAsInt` (`self.BB_PathIndex`)) 1))
  (if (== (`BTFunctionLibrary.GetBlackboardValueAsInt` (`self.BB_Direction`)) 1)
    (bind _asbp_dummy (cast `/Game/Blueprints/BP_Dummy` ControlledPawn))
    (if (<= _returnvalue (- (`KismetArrayLibrary.Array_Length` (`/Game/Blueprints/BP_PatrolPath.PathPoints` (`/Game/Blueprints/BP_Dummy.PatrolPath` _asbp_dummy))) 1))
      ;[1 1 1] Keeps going forward
      (`BTFunctionLibrary.SetBlackboardValueAsInt` _bb_direction 1)
      (`BTFunctionLibrary.SetBlackboardValueAsInt` (`self.BB_PathIndex`) _returnvalue)
      (`self.FinishExecute` true)
      (else
        ;[1 1 1] Starts going reverse
        (`BTFunctionLibrary.SetBlackboardValueAsInt` _bb_direction -1)
        ;[1 1 1] When the path ends
        (`self.FinishExecute` false)))
    (else
      (`self.FinishExecute` false))))