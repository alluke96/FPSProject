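; Behavior tree task that gives a BP_DummyAI its current patrol destination.
; It reads the path index from the blackboard, takes that entry in the AI's PatrolPath PathPoints, converts it from the path actor's local space to world space and writes it to the path vector key.
; It finishes successfully after writing; a failed cast or invalid path never calls FinishExecute.
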(event `self.ReceiveExecuteAI`
  (params (OwnerController :type "AIController Object Reference") (ControlledPawn :type "Pawn Object Reference"))
  (bind _asbp_dummy_ai (cast `/Game/Blueprints/BP_DummyAI` ControlledPawn))
  (bind _patrolpath (`/Game/Blueprints/BP_DummyAI.PatrolPath` _asbp_dummy_ai)
    (:`then`
      (`BTFunctionLibrary.SetBlackboardValueAsVector` (`self.BB_PathVector`) (`KismetMathLibrary.TransformLocation` (`Actor.GetTransform` _patrolpath) (`|GetArrayItem` (`/Game/Blueprints/BP_PatrolPath.PathPoints` _patrolpath) (`BTFunctionLibrary.GetBlackboardValueAsInt` (`self.BB_PathIndex`)))))
      (`self.FinishExecute` true))
    (:`else`)))