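; Behavior Tree task that steps an AI's path index backwards, handling the reverse leg of back-and-forth path movement.
; When the Blackboard direction is reverse, it decrements the path index and succeeds while the result stays non-negative.
; At the path start it flips the direction to forward without changing the index and fails.
; It also fails whenever the direction is not reverse.
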(event `self.ReceiveExecuteAI`
  (params (OwnerController :type "AIController Object Reference") (ControlledPawn :type "Pawn Object Reference"))
  (bind _bb_direction (`self.BB_Direction`))
  (bind _returnvalue (- (`BTFunctionLibrary.GetBlackboardValueAsInt` (`self.BB_PathIndex`)) 1))
  (if (== (`BTFunctionLibrary.GetBlackboardValueAsInt` (`self.BB_Direction`)) -1)
    (if (>= _returnvalue 0)
      ;[1 1 1] Keep going reverse
      (`BTFunctionLibrary.SetBlackboardValueAsInt` _bb_direction -1)
      (`BTFunctionLibrary.SetBlackboardValueAsInt` (`self.BB_PathIndex`) _returnvalue)
      (`self.FinishExecute` true)
      (else
        ;[1 1 1] Start going forward
        (`BTFunctionLibrary.SetBlackboardValueAsInt` _bb_direction 1)
        ;[1 1 1] When the path is back to the start
        (`self.FinishExecute` false)))
    (else
      (`self.FinishExecute` false))))