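; BP_ResetButton is a button actor that replaces the BP_DummyAI targets in the level, on BeginPlay and on demand.
; RestoreDummies destroys each existing dummy and spawns a replacement at a random position within a fixed area, so it only replaces dummies still present.
; Overlapping the button as BP_FPSCharacter enables input and opens a Gate, letting E trigger the reset as an alternative to shooting it.
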(event `self.ReceiveBeginPlay`
  (`self.RestoreDummies`))

(event `RestoreDummies`
  (bind _outactors (`GameplayStatics.GetAllActorsOfClass` "/Game/Blueprints/BP_DummyAI.BP_DummyAI_C" :!label _label))
  (for _array_element _outactors
    (`self.K2_DestroyActor` _array_element)
    (`|SpawnActorFromClass` "/Game/Blueprints/BP_DummyAI.BP_DummyAI_C" (`KismetMathLibrary.MakeTransform` (`KismetMathLibrary.MakeVector` (`KismetMathLibrary.RandomFloatInRange` 0.0 3300.0) (`KismetMathLibrary.RandomFloatInRange` 2500.0 3500.0) 135.0) (struct :`Yaw` 270.0)) "AlwaysSpawn" "OverrideRootScale" null null))
  (`KismetSystemLibrary.PrintString` "Dummies Restored" true true (struct :`R` 0.239596 :`B` 1.0 :`A` 1.0) 3.0))

(event `Key|E`
  (params (Key :type "Key Structure"))
  ;[1 1 1] Caso houver necessidade de apertar o botao com o teclado (sem atirar nele)
  (:`Pressed`
    (`/Engine/EditorBlueprintResources/StandardMacros.Gate` true :!label _label_2
      (:`Exit`
        (goto _label)))))

(event `self.Button.OnComponentBeginOverlap`
  (params (OverlappedComponent :type "PrimitiveComponent Object Reference") (OtherActor :type "Actor Object Reference") (OtherComp :type "PrimitiveComponent Object Reference") (OtherBodyIndex :type Integer) (bFromSweep :type Boolean) (SweepResult :type "HitResult Structure (by ref)"))
  ;[1 1 1] Caso houver necessidade de apertar o botao com o teclado (sem atirar nele)
  (cast `/Game/Blueprints/BP_FPSCHaracter` OtherActor)
  (`self.EnableInput` (`GameplayStatics.GetPlayerController` 0))
  (goto _label_2 :!via `Open`))

(event `self.Button.OnComponentEndOverlap`
  (params (OverlappedComponent :type "PrimitiveComponent Object Reference") (OtherActor :type "Actor Object Reference") (OtherComp :type "PrimitiveComponent Object Reference") (OtherBodyIndex :type Integer))
  ;[1 1 1] Caso houver necessidade de apertar o botao com o teclado (sem atirar nele)
  (cast `/Game/Blueprints/BP_FPSCHaracter` OtherActor)
  (`self.DisableInput` (`GameplayStatics.GetPlayerController` 0))
  (goto _label_2 :!via `Close`))

(fn `UserConstructionScript`)