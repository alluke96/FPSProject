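; Player shotgun weapon Blueprint that overrides raycast firing to shoot multiple pellets, each a visibility line trace using camera-derived start and end points.
; Dummy hits leave blood decals, apply damage inversely proportional to distance when damageable, and add a mesh impulse if dead.
; Reset button hits restore the dummies, while other hits leave temporary bullet holes.
; Tick sets reload time to the number of rounds missing from the clip.
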(event `self.ReceiveTick`
  (params (DeltaSeconds :type "Float (single-precision)"))
  (set `self.ReloadTime` (`KismetMathLibrary.Conv_IntToDouble` (- (`self.MaxClipCapacity`) (`self.CurrentClipAmount`)))))

(fn `FireRaycast`
  (locals (NumberOfPellets :type Integer :default 5))
  (for _ (range (+ (`local.NumberOfPellets`) 1))
    (bind (_start _end) (`self.CameraEquationsForRaycasting`))
    (bind _outhit (`KismetSystemLibrary.LineTraceSingle` :`Start` _start :`End` _end :`TraceChannel` "TraceTypeQuery1" :`DrawTime` 1.0))
    (bind (_bblockinghit _binitialoverlap _time _distance _location _impactpoint _normal _impactnormal _physmat _hitactor _hitcomponent _hitbonename) (`GameplayStatics.BreakHitResult` _outhit))
    (if _bblockinghit
      ;[1 1 1] If it hits a Dummy
      (bind _asbp_dummy_ai (cast `/Game/Blueprints/BP_DummyAI` _hitactor)
        (:`then`
          (bind _returnvalue (`KismetMathLibrary.Conv_VectorToRotator` _impactnormal))
          (`GameplayStatics.SpawnDecalAtLocation` "/Game/Decals/BloodSplat.BloodSplat" (100.0 100.0 100.0) _location _returnvalue)
          (if (`Actor.bCanBeDamaged` _asbp_dummy_ai)
            (`GameplayStatics.ApplyDamage` _hitactor (/ (* (`self.Damage`) 100.0) _distance) null (`self.FPSCharacterRef`))
            (if (`/Game/Blueprints/BP_DummyAI.IsDead` _asbp_dummy_ai)
              (`PrimitiveComponent.AddImpulseAtLocation` (`Character.Mesh` _asbp_dummy_ai) _impactpoint _location _hitbonename))))
        (:`CastFailed`
          ;[1 1 1] If it hits the reset button
          (bind _asbp_reset_button (cast `/Game/Blueprints/BP_ResetButton` _hitactor)
            (:`then`
              (`/Game/Blueprints/BP_ResetButton.RestoreDummies` _asbp_reset_button))
            (:`CastFailed`
              (`GameplayStatics.SpawnDecalAtLocation` "/Game/Decals/BulletHole.BulletHole" (20.0 20.0 20.0) _location _returnvalue 10.0))))))))

(fn `UserConstructionScript`
  (`parent.UserConstructionScript`))