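; Enemy burst rifle weapon that fires hitscan shots in random-sized bursts, with automatic reload on an empty clip.
; StartFiring uses a DoN gate, reset after a delay between bursts, to decrement ammo and call FireRaycast.
; FireRaycast traces forward from the root with debug drawing, applying damage and bullet-hole decals on hits.
; All BP_DummyAI actors are cached at BeginPlay and ignored by the trace to prevent friendly fire.
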(event `self.ReceiveBeginPlay`
  ;[1 1 1] Initialize Enemy Array to disable friendly fire
  (bind _outactors (`GameplayStatics.GetAllActorsOfClass` "/Game/Blueprints/BP_DummyAI.BP_DummyAI_C"))
  (set `self.EnemyArrayToIgnoreInRaycast` _outactors))

(event `StartFiring`
  ;[1 1 1] Fire
  (bind _canshoot (`self.CheckIfCanShoot`))
  (if _canshoot
    (bind _output_get (set `self.NumberOfBulletsInEachBurst` (`KismetMathLibrary.RandomIntegerInRange` 1 5)))
    (bind _counter (`/Engine/EditorBlueprintResources/StandardMacros.Do N` _output_get :!label _label)
      (:`Exit`
        (`self.DecrementClipAmmo`)
        (`self.FireRaycast`)
        (if (== _counter _output_get)
          (`KismetSystemLibrary.Delay` (`self.DelayBetweenBursts`))
          (`self.TurnOffFX&Audio`)
          (goto _label :!via `Reset`))))
    (else
      (`self.TurnOffFX&Audio`))))

(event `Reload`
  ;[1 1 1] Reload
  (set `self.IsReloading` true)
  (`KismetSystemLibrary.Delay` (`self.ReloadTime`))
  (set `self.CurrentClipAmount` (+ (`self.CurrentClipAmount`) (`self.MaxClipCapacity`)))
  (set `self.IsReloading` false))

(fn `CheckIfCanShoot`
  (returns (CanShoot :type Boolean))
  (bind _isreloading (`self.Check If Is Reloading`))
  (if (not _isreloading)
    (bind _clipisempty (`self.CheckIfClipIsEmpty`))
    (if _clipisempty
      (`self.Reload`)
      (return false)
      (else
        (return true)))))

(fn `FireRaycast`
  (bind _root (`self.Root`))
  (bind _returnvalue (`SceneComponent.K2_GetComponentLocation` _root))
  (`self.TurnOnFX&Audio`)
  (bind _outhit (`KismetSystemLibrary.LineTraceSingle` _returnvalue (+ _returnvalue (* (`SceneComponent.GetForwardVector` _root) (`self.WeaponRange`))) "TraceTypeQuery1" false (`self.EnemyArrayToIgnoreInRaycast`) "ForDuration" true (struct :`R` 1.0 :`A` 1.0) (struct :`G` 1.0 :`A` 1.0) 1.0))
  (bind (_bblockinghit _binitialoverlap _time _distance _location _impactpoint _normal _impactnormal _physmat _hitactor) (`GameplayStatics.BreakHitResult` _outhit))
  (if _bblockinghit
    (`GameplayStatics.ApplyDamage` _hitactor (`self.Damage`))
    (`GameplayStatics.SpawnDecalAtLocation` "/Game/Decals/BulletHole.BulletHole" (20.0 20.0 20.0) _location (`KismetMathLibrary.Conv_VectorToRotator` _impactnormal) 10.0)))

(fn `UserConstructionScript`
  (`parent.UserConstructionScript`))