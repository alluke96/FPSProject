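; BP_Weapon is the player's hitscan gun, handling firing, ammo, recoil and reloading through BP_FPSCharacter.
; Fire checks rate and state, then line-traces from the camera (randomly offset for buckshot) to damage dummies, trigger reset buttons or place decals.
; Shots add random recoil and play muzzle and audio effects with AI noise; the timeline recoil is left unbound.
; The character's reload event tilts the mesh, waits, then refills from its holster ammo.
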(event `self.ReceiveBeginPlay`
  ;[1 1 1] Begin
  (bind _fpscharacterref (`self.GetPlayerRef`))
  (bind _output_get (set `self.FPSCharacterRef` _fpscharacterref))
  (add `/Game/Blueprints/BP_FPSCHaracter.OnReload` _output_get (delegate `OnReload_Event`)))

(event `OnReload_Event`
  ;[1 1 1] Begin
  (`self.Reload`))

(event `DoRecoil`
  (bind _returnvalue (`PawnMovementComponent.GetPawnOwner` (`Character.CharacterMovement` (`self.FPSCharacterRef`))))
  ;[1 1 1] TODO Recoil
  (if (`/Game/Blueprints/BP_FPSCHaracter.PressedFire` (`self.FPSCharacterRef`))
    (bind (_direction _rifleyaw _riflepitch) (`Timeline|RecoilPatterns` :!via `PlayFromStart` :!label _label)
      (:`Update`
        (`Pawn.AddControllerYawInput` _returnvalue _rifleyaw)
        (`Pawn.AddControllerPitchInput` _returnvalue _riflepitch)))
    (else
      (goto _label :!via `Stop`))))

(fn `CameraEquationsForRaycasting`
  (returns (Start :type "Vector Structure") (End :type "Vector Structure"))
  (locals (Camera :type "CameraComponent Object Reference"))
  (bind _camera (`local.Camera`))
  (bind _camera_2 (`local.Camera`))
  (bind _returnvalue (`SceneComponent.K2_GetComponentLocation` _camera_2))
  (bind _returnvalue_2 (`SceneComponent.K2_GetComponentLocation` _camera))
  (bind (_returnvalue_x _returnvalue_y _returnvalue_z) (`KismetMathLibrary.BreakVector` (+ _returnvalue_2 (* (`SceneComponent.GetForwardVector` _camera) (`self.WeaponRange`)))))
  (set `local.Camera` (`/Game/Blueprints/BP_FPSCHaracter.Camera` (`self.FPSCharacterRef`)))
  (if (`self.ShouldFireBuckshot`)
    (return _returnvalue_2 (`KismetMathLibrary.MakeVector` _returnvalue_x (+ _returnvalue_y (`KismetMathLibrary.RandomFloatInRange` -600.0 600.0)) (+ _returnvalue_z (`KismetMathLibrary.RandomFloatInRange` -600.0 600.0))))
    (else
      (return _returnvalue (+ _returnvalue (* (`SceneComponent.GetForwardVector` _camera_2) (`self.WeaponRange`)))))))

(fn `Check If Is Reloading`
  (returns (IsReloading :type Boolean))
  (return (== (`self.IsReloading`) true)))

(fn `CheckIfCanReload`
  (returns (CanReload :type Boolean))
  (bind _isreloading (`self.CheckIfPlayerIsRunning`))
  (bind _isreloading_2 (`self.Check If Is Reloading`))
  (bind _clipisfull (`self.CheckIfClipIsFull`))
  (return (and (not _clipisfull) (not _isreloading_2) (not _isreloading))))

(fn `CheckIfClipIsEmpty`
  (returns (ClipIsEmpty :type Boolean))
  (return (<= (`self.CurrentClipAmount`) 0)))

(fn `CheckIfClipIsFull`
  (returns (ClipIsFull :type Boolean))
  (return (>= (`self.CurrentClipAmount`) (`self.MaxClipCapacity`))))

(fn `CheckIfPlayerIsRunning`
  (returns (IsReloading :type Boolean))
  (return (== (`/Game/Blueprints/BP_FPSCHaracter.IsRunning` (`self.FPSCharacterRef`)) true)))

(fn `CheckIfWeaponCanShoot`
  (returns (CanShoot :type Boolean))
  (bind _isreloading (`self.CheckIfPlayerIsRunning`))
  (bind _isreloading_2 (`self.Check If Is Reloading`))
  (bind _clipisempty (`self.CheckIfClipIsEmpty`))
  (if (>= (`KismetSystemLibrary.GetGameTimeInSeconds`) (+ (`/Game/Blueprints/BP_FPSCHaracter.LastShotTime` (`self.FPSCharacterRef`)) (`self.FireRate`)))
    (return (and (not _clipisempty) (not _isreloading_2) (not _isreloading)))))

(fn `DecrementClipAmmo`
  (`/Engine/EditorBlueprintResources/StandardMacros.DecrementInt` (`self.CurrentClipAmount`)))

(fn `Fire`
  (bind _canshoot (`self.CheckIfWeaponCanShoot`))
  (if _canshoot
    (`/Engine/EditorBlueprintResources/StandardMacros.DoOnce` false :!label _label
      (:`Completed`
        (`self.DecrementClipAmmo`)
        (`self.FireRaycast`)
        (`self.StartRecoil`)
        (`self.TurnOnFX&Audio`)
        (goto _label :!via `Reset`)))
    (else
      (`self.TurnOffFX&Audio`))))

(fn `FireRaycast`
  (bind (_start _end) (`self.CameraEquationsForRaycasting`))
  (bind _outhit (`KismetSystemLibrary.LineTraceSingle` :`Start` _start :`End` _end :`TraceChannel` "TraceTypeQuery1" :`DrawTime` 1.0))
  (bind (_bblockinghit _binitialoverlap _time _distance _location _impactpoint _normal _impactnormal _physmat _hitactor) (`GameplayStatics.BreakHitResult` _outhit))
  (if _bblockinghit
    ;[1 1 1] If it hits a Dummy
    (bind _asbp_dummy_ai (cast `/Game/Blueprints/BP_DummyAI` _hitactor)
      (:`then`
        (bind _returnvalue (`KismetMathLibrary.Conv_VectorToRotator` _impactnormal))
        (`GameplayStatics.SpawnDecalAtLocation` "/Game/Decals/BloodSplat.BloodSplat" (100.0 100.0 100.0) _location _returnvalue)
        (if (`Actor.bCanBeDamaged` _asbp_dummy_ai)
          (`GameplayStatics.ApplyDamage` _hitactor (`self.Damage`) null (`self.FPSCharacterRef`))))
      (:`CastFailed`
        ;[1 1 1] If it hits the reset button
        (bind _asbp_reset_button (cast `/Game/Blueprints/BP_ResetButton` _hitactor)
          (:`then`
            (`/Game/Blueprints/BP_ResetButton.RestoreDummies` _asbp_reset_button))
          (:`CastFailed`
            (`GameplayStatics.SpawnDecalAtLocation` "/Game/Decals/BulletHole.BulletHole" (20.0 20.0 20.0) _location _returnvalue 10.0)))))))

(fn `GetPlayerRef`
  (returns (FPSCharacterRef :type "/Game/Blueprints/BP_FPSCHaracter Object Reference"))
  (bind _asbp_fpscharacter (cast `/Game/Blueprints/BP_FPSCHaracter` (`GameplayStatics.GetPlayerPawn` 0)))
  (return _asbp_fpscharacter))

(fn `StartRecoil`
  (bind _fpscharacterref (`self.FPSCharacterRef`))
  (bind _returnvalue (`PawnMovementComponent.GetPawnOwner` (`Character.CharacterMovement` _fpscharacterref)))
  (if (`/Game/Blueprints/BP_FPSCHaracter.IsHoldingFire` _fpscharacterref)
    (`Pawn.AddControllerYawInput` _returnvalue (`KismetMathLibrary.RandomFloatInRange` (`self.MinRightRecoil`) (`self.MaxRightRecoil`)))
    (`Pawn.AddControllerPitchInput` _returnvalue (`KismetMathLibrary.RandomFloatInRange` (`self.MinUpRecoil`) (`self.MaxUpRecoil`)))))

(fn `TurnOffFX&Audio`
  (`|ExecutionSequence`
    (:`then_0`
      (`AudioComponent.Stop` (`self.GunLoopSound`)))
    (:`then_1`
      (`SceneComponent.SetVisibility` (`self.MuzzleFlash`) false false))))

(fn `TurnOnFX&Audio`
  (`|ExecutionSequence`
    (:`then_0`
      (`AudioComponent.Play` (`self.GunLoopSound`) 0.0)
      (`AISense_Hearing.ReportNoiseEvent` (`self.K2_GetActorLocation`) (`self.Loudness`) (`self.FPSCharacterRef`) (`self.MaxSoundRange`) "Noise"))
    (:`then_1`
      (`SceneComponent.SetVisibility` (`self.MuzzleFlash`) true false))))

(fn `UserConstructionScript`)